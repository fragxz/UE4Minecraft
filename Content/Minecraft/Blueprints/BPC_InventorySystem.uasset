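; Player inventory component that manages items, action bar slot selection and the held item in a Minecraft-style game.
; AddItem appends items while the length check against TotalActionBarSlots passes, then updates the HUD action bar and re-equips.
; Slot selection wraps on next/previous, updates the HUD and calls EquipItem, which respawns the active item's actor on the Mesh2P Item_Socket.
; Stacking logic is disconnected, and RemoveItem and DropItem are empty.
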(event EventBeginPlay
  (bind _asbp_player (Utilities|Casting|CastToBP_Player (Components|GetOwner)))
  (Variables|Default|SetPlayerCharacterReference _asbp_player)
  (for _array_element (Variables|Default|GetInventory)
    _))

(event EventTick
  (params (DeltaSeconds :type Float%20%28single-precision%29)))

(fn AddItem
  (params (NewItem :type F%20Inventory%20Item%20Structure))
  (if (<= (Utilities|Array|Length (Variables|Default|GetInventory)) (Variables|Settings|GetTotalActionBarSlots))
    (bind _returnvalue (Utilities|Array|Add (Variables|Default|GetInventory) NewItem))
    (Default|UpdateSlot (Variables|/Game/Minecraft/Blueprints/Widgets/WBP_Hud.WBP_HUD_C|GetWBP_ActionBar (Variables|/Game/Minecraft/Blueprints/BP_Player.BP_Player_C|GetHUDReference (Variables|Default|GetPlayerCharacterReference))) _returnvalue (.Item (Utilities|Struct|BreakFInventoryItem NewItem)))
    (CallFunction|EquipItem)))

(fn RemoveItem)

(fn DropItem)

(fn EquipItem
  (bind _activeslot (Variables|Default|GetActiveSlot))
  (bind _inventory (Variables|Default|GetInventory))
  (bind _output (Utilities|Array|Get(acopy) _inventory _activeslot))
  (bind _item (Utilities|Struct|BreakFInventoryItem _output))
  (Utilities|IsValid (Variables|Default|GetEquippedItem)
    (:Is%20Valid
      (Actor|DestroyActor (Variables|Default|GetEquippedItem)))
    (:Is%20Not%20Valid
      _))
  (if (Utilities|Array|IsValidIndex _inventory _activeslot)
    (bind _returnvalue (Game|SpawnActorfromClass (.blueprint _item) (Transformation|GetActorTransform (Variables|Default|GetPlayerCharacterReference)) "Undefined" 0 0))
    (Components|StaticMesh|SetStaticMesh (Variables|/Game/Minecraft/Blueprints/BP_ItemBase.BP_ItemBase_C|GetMesh _returnvalue) (.mesh _item))
    (Rendering|Material|SetMaterial (Variables|/Game/Minecraft/Blueprints/BP_ItemBase.BP_ItemBase_C|GetMesh _returnvalue) 0 (.material _item))
    (Variables|Default|SetEquippedItem _returnvalue)
    (Transformation|AttachComponentToComponent (Variables|Default|GetEquippedItem) (Variables|/Game/Minecraft/Blueprints/BP_Player.BP_Player_C|GetMesh2P (Variables|Default|GetPlayerCharacterReference)) "Item_Socket" "SnapToTarget" "SnapToTarget" "KeepRelative" true)))

(fn SelectNextSlot
  (if (== (Variables|Default|GetActiveSlot) (- (Variables|Settings|GetTotalActionBarSlots) 1))
    (Variables|Default|SetActiveSlot 0)
    (else
      (Math|Integer|IncrementInt (Variables|Default|GetActiveSlot)
        (:%20%20
          _))))
  (CallFunction|SetActiveItemSlot (Variables|Default|GetActiveSlot)))

(fn SelectPreviousSlot
  (if (== (Variables|Default|GetActiveSlot) 0)
    (Variables|Default|SetActiveSlot (- (Variables|Settings|GetTotalActionBarSlots) 1))
    (else
      (Math|Integer|DecrementInt (Variables|Default|GetActiveSlot)
        (:%20%20
          _))))
  (CallFunction|SetActiveItemSlot (Variables|Default|GetActiveSlot)))

(fn SetActiveItemSlot
  (params (NewActiveSlot :type Integer))
  (Development|PrintString (Utilities|String|ToString(Integer) NewActiveSlot))
  (Default|SetActiveSlot (Variables|/Game/Minecraft/Blueprints/Widgets/WBP_Hud.WBP_HUD_C|GetWBP_ActionBar (Variables|/Game/Minecraft/Blueprints/BP_Player.BP_Player_C|GetHUDReference (Variables|Default|GetPlayerCharacterReference))) NewActiveSlot)
  (CallFunction|EquipItem))

(fn GetEquippedItem
  (return (.Item (Utilities|Struct|BreakFInventoryItem (Utilities|Array|Get(acopy) (Variables|Default|GetInventory) (Variables|Default|GetActiveSlot))))))

(fn SelectSlot
  (params (ActiveSlot :type Integer))
  (bind _output_get (Variables|Default|SetActiveSlot ActiveSlot))
  (CallFunction|SetActiveItemSlot _output_get))