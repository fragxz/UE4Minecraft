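; Usable item actor that places a block in the world, in a Minecraft-style game.
; Its Use event calls PlaceBlockActorFromInventory, which spawns the block Blueprint class of the item equipped in the player's inventory component.
; The spawn position is the player's hit block location offset along the hit normal by that block's scaled mesh bounds, so the new block sits against the targeted face.
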(event EventBeginPlay
  (|CallParentFunction) ; This node is disabled and will not be called.\nDrag off pins to build functionality.
)

(event Collision|EventActorBeginOverlap
  (params (OtherActor :type Actor%20Object%20Reference))
  (|CallParentFunction OtherActor) ; This node is disabled and will not be called.\nDrag off pins to build functionality.
)

(event EventTick
  (params (DeltaSeconds :type Float%20%28single-precision%29))
  (|CallParentFunction DeltaSeconds) ; This node is disabled and will not be called.\nDrag off pins to build functionality.
)

(event EventUse
  (CallFunction|PlaceBlockActorfromInventory))

(fn ConstructionScript
  (|CallParentFunction))

(fn PlaceBlockActorfromInventory
  (bind _playercharacterreference (Variables|Default|GetPlayerCharacterReference))
  (bind _hitblock (Variables|/Game/Minecraft/Blueprints/BP_Player.BP_Player_C|GetHitBlock _playercharacterreference))
  ;[0.4531 1 0 0.5] Place Block
  (Game|SpawnActorfromClass (.blockactor_blueprint (Default|GetEquippedItem (Variables|/Game/Minecraft/Blueprints/BP_Player.BP_Player_C|GetBPC_InventorySystem (Variables|Default|GetPlayerCharacterReference)))) (Math|Conversions|ToTransform(Vector) (+ (Transformation|GetActorLocation _hitblock) (* (Variables|/Game/Minecraft/Blueprints/BP_Player.BP_Player_C|GetHitNormal _playercharacterreference) (CallFunction|GetScaledStaticMeshBounds (Variables|/Game/Minecraft/Blueprints/BP_Block.BP_Block_C|GetCube _hitblock))))) "Undefined" 0 0))